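; BP_RadiationZone is a spherical anomaly that irradiates the player character while they are inside it.
; Overlapping the sphere caches the BP_MyCharacter and starts a looping timer, and leaving clears both.
; TakeRadiation sends a dose to the character's BPCRadiation component, scaled by zone strength and timer interval.
; The dose follows a quadratic falloff, strongest at the center and zero at the sphere's edge.
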(event `self.Sphere.OnComponentBeginOverlap`
  (params (OverlappedComponent :type "PrimitiveComponent Object Reference") (OtherActor :type "Actor Object Reference") (OtherComp :type "PrimitiveComponent Object Reference") (OtherBodyIndex :type Integer) (bFromSweep :type Boolean) (SweepResult :type "HitResult Structure (by ref)"))
  (bind _asbp_my_character (cast `/Game/MyCharacter/Blueprints/BP_MyCharacter` OtherActor))
  (set `self.As BP My Character` _asbp_my_character)
  (bind _returnvalue (`KismetSystemLibrary.K2_SetTimerDelegate` (`|CreateDelegate` :!event `TakeRadiation`) (`self.TimeLoppingTimer`) true))
  (set `self.TimerTakeRadiation` _returnvalue))

(event `self.Sphere.OnComponentEndOverlap`
  (params (OverlappedComponent :type "PrimitiveComponent Object Reference") (OtherActor :type "Actor Object Reference") (OtherComp :type "PrimitiveComponent Object Reference") (OtherBodyIndex :type Integer))
  (cast `/Game/MyCharacter/Blueprints/BP_MyCharacter` OtherActor)
  (set `self.As BP My Character` null)
  (`KismetSystemLibrary.K2_ClearAndInvalidateTimerHandle` (`self.TimerTakeRadiation`)))

(fn `TakeRadiation`
  (bind _sphere (`self.Sphere`))
  (bind _as_bp_my_character (`self.As BP My Character`)
    (:`then`
      (`/Game/MyCharacter/Blueprints/BPC_Radiation.TakeRadiation` (`/Game/MyCharacter/Blueprints/BP_MyCharacter.BPC_Radiation` _as_bp_my_character) (/ (* (`self.RadoationStrength_mSv`) (- 1.0 (`KismetMathLibrary.MultiplyMultiply_FloatFloat` (`KismetMathLibrary.FClamp` (/ (`KismetMathLibrary.VSize` (- (`SceneComponent.K2_GetComponentLocation` (`Character.CapsuleComponent` (`self.As BP My Character`))) (`SceneComponent.K2_GetComponentLocation` _sphere))) (`SphereComponent.SphereRadius` _sphere))) 2.0)) (`self.TimeLoppingTimer`)) 100.0)))
    (:`else`)))

(fn `UserConstructionScript`)