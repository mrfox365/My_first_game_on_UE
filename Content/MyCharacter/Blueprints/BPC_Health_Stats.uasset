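; Player survival component for BP_MyCharacter that tracks health, stamina, hunger and thirst, creates the stats HUD, and handles death and respawn.
; Looping timers drain hunger and thirst and apply passive healing, while Tick handles sprint stamina, delayed recovery and active health regen.
; Hunger and thirst levels adjust regen multipliers or deal damage at zero, and consumable-style functions grant instant refills or timed buffs.
; Death ragdolls the character and shows a respawn screen; respawn restarts the player through the GameMode.
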(event `self.ReceiveBeginPlay`
  (`|ExecutionSequence`
    (:`then_0`
      (bind _asbp_my_character (cast `/Game/MyCharacter/Blueprints/BP_MyCharacter` (`self.GetOwner`)))
      (set `self.As BP My Character` _asbp_my_character)
      (set `self.GameMode` (`GameplayStatics.GetGameMode`))
      (set `self.PlayerController` (`GameplayStatics.GetPlayerController` 0)))
    (:`then_1`
      (`self.Set HP_SM` 100.0 100.0 100.0 100.0)
      (`self.Set HG_TH` 100.0 40.0 100.0 40.0))
    (:`then_2`
      (`KismetSystemLibrary.K2_SetTimerDelegate` (`|CreateDelegate` :!event ` Handle Decrease Hunger`) (`self.TimerDecreaseHG`) true)
      (`KismetSystemLibrary.K2_SetTimerDelegate` (`|CreateDelegate` :!event `Handle Decrease Thirst`) (`self.TimerDecreaseTH`) true)
      (`KismetSystemLibrary.K2_SetTimerDelegate` (`|CreateDelegate` :!event `Passive Health Regeneration`) (`self.TimerPRegenerationHP`) true))
    (:`then_3`
      (bind _returnvalue (`|CreateWidget` "/Game/UI/Stats_HUD.Stats_HUD_C"))
      (bind _output_get (set `self.Stats_HUD` _returnvalue))
      (`UserWidget.AddToViewport` _output_get 0))
    (:`then_4`
      (bind _returnvalue_2 (`|CreateWidget` "/Game/UI/Respawn_HUD.Respawn_HUD_C"))
      (set `self.Respawn_HUD` _returnvalue_2))))

(event `Waste Stamina Jump`
  ;[0.05127 0.05127 0.05127] Waste Stamina Jump
  (set `self.CurrentSM` (`KismetMathLibrary.FClamp` (- (`self.CurrentSM`) (`self.JumpWasteSM`)) 0.0 (`self.MaxSM`)))
  (set `self.CurrentSMTimerRecover` 0.0 :!label _label))

(event `self.ReceiveTick`
  (params (DeltaSeconds :type "Float (single-precision)"))
  (bind _timerbuffstaminaregen (`self.TimerBuffStaminaRegen`))
  (bind _returnvalue (`KismetSystemLibrary.K2_GetTimerRemainingTimeHandle` _timerbuffstaminaregen))
  (`|ExecutionSequence`
    (:`then_0`
      (if (and (> (`KismetMathLibrary.VSize` (`Actor.GetVelocity` (`self.GetOwner`))) 200.0) (`/Game/MyCharacter/Blueprints/BP_MyCharacter.isRunning` (`self.As BP My Character`)))
        (if (> (`self.CurrentSM`) 0.0)
          ;[0.05127 0.05127 0.05127] Waste Stamina Sprint
          (set `self.CurrentSM` (`KismetMathLibrary.FClamp` (- (`self.CurrentSM`) (* (`self.SpeedWasteSM`) DeltaSeconds)) 0.0 (`self.MaxSM`)))
          (goto _label)
          (else
            (set `/Game/MyCharacter/Blueprints/BP_MyCharacter.canWasteStamina` false (`self.As BP My Character`))))
        (elif (< (`self.CurrentSM`) (`self.MaxSM`))
          (if (>= (`self.CurrentSMTimerRecover`) (`self.SMTimerRecover`))
            ;[0.05127 0.05127 0.05127] Recover Stamina
            (bind _output_get (set `self.CurrentSM` (`KismetMathLibrary.FClamp` (+ (`self.CurrentSM`) (* (`self.SpeedRecoverSM`) DeltaSeconds (`self.MultiplySpeedRecoverSM`))) 0.0 (`self.MaxSM`))))
            (if (`/Game/MyCharacter/Blueprints/BP_MyCharacter.canWasteStamina` (`self.As BP My Character`))
              _
              (elif (> _output_get (/ (`self.MaxSM`) 2.0))
                (set `/Game/MyCharacter/Blueprints/BP_MyCharacter.canWasteStamina` true (`self.As BP My Character`))))
            (else
              ;[0.05127 0.05127 0.05127] Stamina Timer
              (set `self.CurrentSMTimerRecover` (+ DeltaSeconds (`self.CurrentSMTimerRecover`))))))))
    (:`then_1`
      (if (`KismetSystemLibrary.K2_IsTimerActiveHandle` (`self.TimerBuffHealthRegen`))
        (if (< (`self.CurrentHP`) (`self.MaxHP`))
          (set `self.CurrentHP` (+ (`self.CurrentHP`) (* (`self.SpeedRecoverHP`) DeltaSeconds))))))
    (:`then_2`
      (if (`KismetSystemLibrary.K2_IsTimerActiveHandle` (`self.TimerBuffStaminaRegen`))
        (bind _staminabuffwidget (`self.StaminaBuffWidget`)
          (:`then`
            (`/Game/UI/StaminaBuff.ChangePercent` _staminabuffwidget (/ _returnvalue (+ (`KismetSystemLibrary.K2_GetTimerElapsedTimeHandle` _timerbuffstaminaregen) _returnvalue))))
          (:`else`))))))

(event `Dead`
  (bind _respawn_hud (`self.Respawn_HUD`))
  (bind _mesh (`Character.Mesh` (`self.As BP My Character`)))
  (bind _ui_inventory (`/Game/MyCharacter/Blueprints/Inventory/BPC_Inventory.UI_Inventory` (`/Game/MyCharacter/Blueprints/BP_MyCharacter.BPC_Invemtory` (`self.As BP My Character`))))
  (set `self.isDead` true)
  (`GameplayStatics.PlaySound2D` "/Game/Sounds/Death/man-death_Cue.man-death_Cue" 1.0 1.0 0.0 null null)
  (`CharacterMovementComponent.DisableMovement` (`Character.CharacterMovement` (`self.As BP My Character`)))
  (`SceneComponent.K2_DetachFromComponent` (`/Game/MyCharacter/Blueprints/BP_MyCharacter.FirstPersonCamera` (`self.As BP My Character`)) "KeepWorld" "KeepRelative" "KeepRelative" false)
  (`PrimitiveComponent.SetCollisionProfileName` _mesh "Ragdoll" true)
  (`PrimitiveComponent.SetSimulatePhysics` _mesh true)
  (`Widget.RemoveFromParent` (`self.Stats_HUD`))
  (`/Engine/EditorBlueprintResources/StandardMacros.IsValid` _ui_inventory
    (:`Is Valid`
      (`Widget.RemoveFromParent` _ui_inventory))
    (:`Is Not Valid`
      _))
  (`Widget.RemoveFromParent` (`/Game/MyCharacter/Blueprints/BP_MyCharacter.Tips_HUD` (`self.As BP My Character`)))
  (`UserWidget.AddToViewport` _respawn_hud 0)
  (`/Game/UI/Respawn_HUD.Death on HUD BP` _respawn_hud))

(event `Respawn`
  (set `self.isDead` false)
  (`Widget.RemoveFromParent` (`self.Respawn_HUD`))
  (`Pawn.DetachFromControllerPendingDestroy` (`self.As BP My Character`))
  (`Actor.K2_DestroyActor` (`self.As BP My Character`))
  (`GameModeBase.RestartPlayer` (`self.GameMode`) (`self.PlayerController`)))

(fn ` Handle Decrease Hunger`
  (if (> (`self.CurrentHG`) 0.0)
    (bind _output_get (set `self.CurrentHG` (`KismetMathLibrary.FClamp` (- (`self.CurrentHG`) (* (`self.SpeedWasteHG`) (`self.TimerDecreaseHG`) (`self.MultiplySpeedWasteHG`))) 0.0 (`self.MaxHG`))))
    (set `self.isHungry` false)
    (if (>= _output_get (/ (`self.MaxHG`) 2.0))
      (if (not (`self.isChangeMultiply_InHG`))
        (set `self.isChangeMultiply_InHG` true)
        (set `self.MultiplySpeedRecoverSM` (+ (`self.MultiplySpeedRecoverSM`) (`self.IncriseMultiplySpeedRecoverSM_HG_MoreHalf`))))
      (elif (`self.isChangeMultiply_InHG`)
        (set `self.isChangeMultiply_InHG` false)
        (set `self.MultiplySpeedRecoverSM` (- (`self.MultiplySpeedRecoverSM`) (`self.IncriseMultiplySpeedRecoverSM_HG_MoreHalf`)))))
    (else
      ;[1 1 1] Damage then hungry
      (`GameplayStatics.ApplyDamage` (`self.As BP My Character`) (* (`self.DamageHungry`) (`self.TimerDecreaseHG`)))
      (set `self.isHungry` true))))

(fn `Buff Ended Health Regen`
  (set `self.SpeedRecoverHP` (- (`self.SpeedRecoverHP`) (`self.OldBuffHealthRegen`))))

(fn `Buff Ended Stamina Regen`
  (set `self.MultiplySpeedRecoverSM` (- (`self.MultiplySpeedRecoverSM`) (`self.OldBuffStaminaRegen`)))
  (bind _staminabuffwidget (`self.StaminaBuffWidget`)
    (:`then`
      (`Widget.RemoveFromParent` _staminabuffwidget)
      (set `self.StaminaBuffWidget` null))
    (:`else`)))

(fn `Buff Health Regen`
  (params (BaffRegenHealth :type "Float (double-precision)") (TimeBaff :type "Float (double-precision)"))
  (returns (`IsUse?` :type Boolean))
  (bind _timerbuffhealthregen (`self.TimerBuffHealthRegen`))
  (bind _returnvalue (`KismetSystemLibrary.K2_GetTimerRemainingTimeHandle` _timerbuffhealthregen))
  (if (`KismetSystemLibrary.K2_IsValidTimerHandle` (`self.TimerBuffHealthRegen`))
    (if (`KismetSystemLibrary.K2_IsTimerActiveHandle` (`self.TimerBuffHealthRegen`))
      (if (< (/ _returnvalue (+ (`KismetSystemLibrary.K2_GetTimerElapsedTimeHandle` _timerbuffhealthregen) _returnvalue)) 0.95)
        (`KismetSystemLibrary.K2_ClearAndInvalidateTimerHandle` (`self.TimerBuffHealthRegen`))
        (`self.Buff Ended Health Regen`)
        (else
          (return false)))))
  (bind _returnvalue_2 (`KismetSystemLibrary.K2_SetTimerDelegate` (`|CreateDelegate` :!event `Buff Ended Health Regen`) (`local.TimeBaff`)))
  (set `self.TimerBuffHealthRegen` _returnvalue_2)
  (set `self.SpeedRecoverHP` (+ (`self.SpeedRecoverHP`) (`local.BaffRegenHealth`)))
  (set `self.OldBuffHealthRegen` (`local.BaffRegenHealth`))
  (return true))

(fn `Buff Stamina Regen`
  (params (BaffRegenMultiply :type "Float (double-precision)") (TimeBaff :type "Float (double-precision)"))
  (returns (`isUse?` :type Boolean))
  (bind _timerbuffstaminaregen (`self.TimerBuffStaminaRegen`))
  (bind _returnvalue (`KismetSystemLibrary.K2_GetTimerRemainingTimeHandle` _timerbuffstaminaregen))
  (if (`KismetSystemLibrary.K2_IsValidTimerHandle` (`self.TimerBuffStaminaRegen`))
    (if (`KismetSystemLibrary.K2_IsTimerActiveHandle` (`self.TimerBuffStaminaRegen`))
      (if (< (/ _returnvalue (+ (`KismetSystemLibrary.K2_GetTimerElapsedTimeHandle` _timerbuffstaminaregen) _returnvalue)) 0.95)
        (`KismetSystemLibrary.K2_ClearAndInvalidateTimerHandle` (`self.TimerBuffStaminaRegen`))
        (`self.Buff Ended Stamina Regen`)
        (else
          (return false)))))
  (bind _returnvalue_2 (`KismetSystemLibrary.K2_SetTimerDelegate` (`|CreateDelegate` :!event `Buff Ended Stamina Regen`) (`local.TimeBaff`)))
  (set `self.TimerBuffStaminaRegen` _returnvalue_2)
  (set `self.MultiplySpeedRecoverSM` (+ (`self.MultiplySpeedRecoverSM`) (`local.BaffRegenMultiply`)))
  (set `self.OldBuffStaminaRegen` (`local.BaffRegenMultiply`))
  (bind _returnvalue_3 (`|CreateWidget` "/Game/UI/StaminaBuff.StaminaBuff_C"))
  (bind _output_get (set `self.StaminaBuffWidget` _returnvalue_3))
  (`/Game/UI/BuffGrid.AddBuff` (`/Game/UI/Stats_HUD.BuffGrid` (`self.Stats_HUD`)) _output_get)
  (return true))

(fn `Do Damage`
  (params (Damage :type "Float (double-precision)"))
  (bind _currenthp (`self.CurrentHP`))
  (if (not (`self.isDead`))
    (bind _output_get (set `self.CurrentHP` (`KismetMathLibrary.FClamp` (- _currenthp Damage) 0.0 _currenthp)))
    (if (<= _output_get 0.0)
      (`self.Dead`)
      (elif (>= (`GameplayStatics.GetTimeSeconds`) (+ (`self.Timer_PlayDamageSound`) 3.0))
        (if (`KismetMathLibrary.RandomBoolWithWeight` (`KismetMathLibrary.FClamp` (/ (`local.Damage`) 20.0)))
          (`GameplayStatics.PlaySound2D` "/Game/Sounds/TakeDamade/take-damage_Cue.take-damage_Cue" 1.0 1.0 0.0 null null)
          (set `self.Timer_PlayDamageSound` (`GameplayStatics.GetTimeSeconds`)))))))

(fn `Get Stats for HG_TH_HUD`
  (returns (`Progress Bar HG` :type "Float (double-precision)") (`Progress Bar TH` :type "Float (double-precision)"))
  (return (`KismetMathLibrary.NormalizeToRange` (`self.CurrentHG`) 0.0 (`self.MaxHG`)) (`KismetMathLibrary.NormalizeToRange` (`self.CurrentTH`) 0.0 (`self.MaxTH`))))

(fn `Get Stats for HP_SM_HUD`
  (returns (`Progress Bar HP` :type "Float (double-precision)") (`Progress Bar HP Last Regen` :type "Float (double-precision)") (`Progress Bar SM` :type "Float (double-precision)"))
  (locals (LastRegenHP :type "Float (double-precision)"))
  (bind _timerbuffhealthregen (`self.TimerBuffHealthRegen`))
  (if (`KismetSystemLibrary.K2_IsValidTimerHandle` _timerbuffhealthregen)
    (if (`KismetSystemLibrary.K2_IsTimerActiveHandle` _timerbuffhealthregen)
      (set `local.LastRegenHP` (+ (`self.CurrentHP`) (* (`self.SpeedRecoverHP`) (`KismetSystemLibrary.K2_GetTimerRemainingTimeHandle` _timerbuffhealthregen))))
      (else
        (set `local.LastRegenHP` 0.0 :!label _label)))
    (else
      (goto _label)))
  (return (`KismetMathLibrary.NormalizeToRange` (`self.CurrentHP`) 0.0 (`self.MaxHP`)) (`KismetMathLibrary.NormalizeToRange` (`local.LastRegenHP`) 0.0 (`self.MaxHP`)) (`KismetMathLibrary.NormalizeToRange` (`self.CurrentSM`) 0.0 (`self.MaxSM`))))

(fn `Handle Decrease Thirst`
  (if (> (`self.CurrentTH`) 0.0)
    (bind _output_get (set `self.CurrentTH` (`KismetMathLibrary.FClamp` (- (`self.CurrentTH`) (* (`self.SpeedWasteTH`) (`self.TimerDecreaseTH`) (`self.MultiplySpeedWasteTH`))) 0.0 (`self.MaxTH`))))
    (set `self.isThirsty` false)
    (if (>= _output_get (/ (`self.MaxTH`) 2.0))
      (if (not (`self.isChangeMultiply_InTH`))
        (set `self.isChangeMultiply_InTH` true)
        (set `self.MultiplySpeedPRegenerationHP` (+ (`self.MultiplySpeedPRegenerationHP`) (`self.IncreaseMultSpeedPRegenHP_TH_MoreHalf`)))
        (set `self.MultiplySpeedRecoverSM` (+ (`self.MultiplySpeedRecoverSM`) (`self.IncriseMultiplySpeedRecoverSM_TH_MoreHalf`))))
      (elif (`self.isChangeMultiply_InTH`)
        (set `self.isChangeMultiply_InTH` false)
        (set `self.MultiplySpeedPRegenerationHP` (- (`self.MultiplySpeedPRegenerationHP`) (`self.IncreaseMultSpeedPRegenHP_TH_MoreHalf`)))
        (set `self.MultiplySpeedRecoverSM` (- (`self.MultiplySpeedRecoverSM`) (`self.IncriseMultiplySpeedRecoverSM_TH_MoreHalf`)))))
    (else
      ;[1 1 1] Damage then thirsty
      (`GameplayStatics.ApplyDamage` (`self.As BP My Character`) (* (`self.DamageThirsty`) (`self.TimerDecreaseHG`)))
      (set `self.isThirsty` true))))

(fn `InstHealth Regen`
  (params (InstHealthRegen :type "Float (double-precision)"))
  (returns (IsUse :type Boolean))
  (if (< (`self.CurrentHP`) (`self.MaxHP`))
    (set `self.CurrentHP` (`KismetMathLibrary.FClamp` (+ (`self.CurrentHP`) (`local.InstHealthRegen`)) 0.0 (`self.MaxHP`)))
    (return true)
    (else
      (return false))))

(fn `InstHunger Regen`
  (params (`InstHunger Regen` :type "Float (double-precision)"))
  (returns (`isUse?` :type Boolean))
  (if (< (`self.CurrentHG`) (* (`self.MaxHG`) 0.95))
    (set `self.CurrentHG` (`KismetMathLibrary.FClamp` (+ (`self.CurrentHG`) (`local.InstHunger Regen`)) 0.0 (`self.MaxHG`)))
    (return true)
    (else
      (return false))))

(fn `InstStamina Regen`
  (params (InstStaminaRegen :type "Float (double-precision)"))
  (returns (`isUse?` :type Boolean))
  (if (< (`self.CurrentSM`) (* (`self.MaxSM`) 0.95))
    (set `self.CurrentSM` (`KismetMathLibrary.FClamp` (+ (`self.CurrentSM`) (`local.InstStaminaRegen`)) 0.0 (`self.MaxSM`)))
    (return true)
    (else
      (return false))))

(fn `InstThirst Regen`
  (params (InstThirstRegen :type "Float (double-precision)"))
  (returns (`isUse?` :type Boolean))
  (if (< (`self.CurrentTH`) (* (`self.MaxTH`) 0.95))
    (set `self.CurrentTH` (`KismetMathLibrary.FClamp` (+ (`self.CurrentTH`) (`local.InstThirstRegen`)) 0.0 (`self.MaxTH`)))
    (return true)
    (else
      (return false))))

(fn `Passive Health Regeneration`
  (`|ExecutionSequence`
    (:`then_1`
      (if (and (< (`self.CurrentHP`) (`self.MaxHP`)) (>= (`self.CurrentHG`) (/ (`self.MaxHG`) 2.0)))
        (set `self.CurrentHP` (`KismetMathLibrary.FClamp` (+ (`self.CurrentHP`) (* (`self.SpeedPRegenerationHP`) (`self.TimerPRegenerationHP`) (`self.MultiplySpeedPRegenerationHP`))) 0.0 (`self.MaxHP`)))
        (if (not (`self.IsPRegenerationHP`))
          (set `self.IsPRegenerationHP` true)
          (set `self.MultiplySpeedWasteHG` (+ (`self.MultiplySpeedWasteHG`) (`self.IncreaseMultSpeedHG_ifReg`))))
        (elif (`self.IsPRegenerationHP`)
          (set `self.IsPRegenerationHP` false)
          (set `self.MultiplySpeedWasteHG` (- (`self.MultiplySpeedWasteHG`) (`self.IncreaseMultSpeedHG_ifReg`))))))))

(fn `Set HG_TH`
  (params (`Set Max HG` :type "Float (double-precision)") (`Set Current HG` :type "Float (double-precision)") (`Set Max TH` :type "Float (double-precision)") (`Set Current TH` :type "Float (double-precision)"))
  (set `self.MaxHG` `Set Max HG`)
  (set `self.CurrentHG` `Set Current HG`)
  (set `self.MaxTH` `Set Max TH`)
  (set `self.CurrentTH` `Set Current TH`))

(fn `Set HP_SM`
  (params (`Set Max HP` :type "Float (double-precision)") (`Set Current HP` :type "Float (double-precision)") (`Set Max SM` :type "Float (double-precision)") (`Set Current SM` :type "Float (double-precision)"))
  (set `self.MaxHP` `Set Max HP`)
  (set `self.CurrentHP` `Set Current HP`)
  (set `self.MaxSM` `Set Max SM`)
  (set `self.CurrentSM` `Set Current SM`))