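; BP_Bandage is a usable inventory item that heals the player who uses it.
; Its UseItem override calls the parent, then applies instant health regeneration through the player's health stats component.
; If that succeeds, it also applies a timed regeneration buff and removes one bandage from the stack through the inventory component.
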(fn `UseItem`
  (params (ItemObject :type "/Game/MyCharacter/Blueprints/Inventory/BP_BaseItemObject Object Reference") (PlayerCharacter :type "/Game/MyCharacter/Blueprints/BP_MyCharacter Object Reference"))
  (bind _bpc_health_stats (`/Game/MyCharacter/Blueprints/BP_MyCharacter.BPC_Health_Stats` (`local.PlayerCharacter`)))
  (`parent.UseItem` ItemObject PlayerCharacter)
  (bind _isuse (`/Game/MyCharacter/Blueprints/BPC_Health_Stats.InstHealth Regen` _bpc_health_stats (`self.InstHealthRegen`)))
  (if _isuse
    (bind _isuse_ (`/Game/MyCharacter/Blueprints/BPC_Health_Stats.Buff Health Regen` _bpc_health_stats (`self.BaffHealthRegen`) (`self.TimeBuff`)))
    (if (or _isuse_ _isuse)
      (`/Game/MyCharacter/Blueprints/Inventory/BPC_Inventory.DecreaseAmount` (`/Game/MyCharacter/Blueprints/BP_MyCharacter.BPC_Invemtory` (`local.PlayerCharacter`)) (`local.ItemObject`) 1))))

(fn `UserConstructionScript`
  (`parent.UserConstructionScript`))