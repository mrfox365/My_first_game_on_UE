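; BP_BaseItemObject is the base data object for an inventory item, holding its dimensions, icon, class, item info and current amount.
; Getters expose these values, with stackability, weight and max stack size read from the ItemInfo struct.
; Rotation is a toggled flag that makes GetItemDimencion return X and Y swapped, leaving the stored Dimension unchanged.
; SetAmount stores the amount without clamping it to the stack limit.
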(fn `GetAmount`
  (returns (Amount :type Integer))
  (return (`self.Amount`)))

(fn `GetIsRotate?`
  (returns (`isRotate?` :type Boolean))
  (return (`self.isRotate?`)))

(fn `GetIsStack?`
  (returns (`IsStack?` :type Boolean))
  (return (`.IsStack?_24_536F9AB94E266AE7FBCF0CB67610BE0E` (break `/Game/MyCharacter/Blueprints/Inventory/ItemInfo` (`self.ItemInfo`)))))

(fn `GetItemClass`
  (returns (ItemClass :type "/Game/MyCharacter/Blueprints/Inventory/BP_BaseInventoryItem Class Reference"))
  (return (`self.ItemClass`)))

(fn `GetItemDimencion`
  (returns (Dimension :type "IntPoint Structure"))
  (bind (_dimension_x _dimension_y) (break `IntPoint` (`self.Dimension`)))
  (if (`self.isRotate?`)
    (return (make `IntPoint` _dimension_y _dimension_x))
    (else
      (return (`self.Dimension`)))))

(fn `GetItemIcon`
  (returns (Icon :type "Texture2D Object Reference"))
  (return (`self.Icon`)))

(fn `GetItemInfo`
  (returns (ItemInfo :type "/Game/MyCharacter/Blueprints/Inventory/ItemInfo Structure"))
  (return (`self.ItemInfo`)))

(fn `GetMaxAmount`
  (returns (MaxAmount :type Integer))
  (return (`.MaxStackAmount_21_0373732445B1E79F487FFFA0D3ADD1BD` (break `/Game/MyCharacter/Blueprints/Inventory/ItemInfo` (`self.ItemInfo`)))))

(fn `GetWeight`
  (returns (Weight :type "Float (double-precision)"))
  (return (`.Weight_9_6391630A4F07430DFD6ED0B2ED93D051` (break `/Game/MyCharacter/Blueprints/Inventory/ItemInfo` (`self.ItemInfo`)))))

(fn `RotateIcon`
  (set `self.isRotate?` (not (`self.isRotate?`)))
  (return))

(fn `SetAmount`
  (params (Amount :type Integer))
  (set `self.Amount` Amount)
  (return))