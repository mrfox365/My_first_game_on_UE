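; BP_BaseInventoryItem is the base world pickup for an inventory item that has grid dimensions and a stack amount.
; On BeginPlay it builds a BP_BaseItemObject from its own properties and class if ItemObject is not already valid.
; Interact offers that object to an InventoryComponent with stacking, destroying the actor when fully absorbed, otherwise setting the leftover amount.
; UseItem is an empty stub at this level.
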(event `self.ReceiveBeginPlay`
  (if (not (`KismetSystemLibrary.IsValid` (`self.ItemObject`)))
    (bind _itemobject (`self.GetDefaultItemObject`))
    (set `self.ItemObject` _itemobject)))

(event `/Game/MyCharacter/Blueprints/Inventory/BPI_interact.Interact`
  (params (InventoryComponent :type "/Game/MyCharacter/Blueprints/Inventory/BPC_Inventory Object Reference"))
  (bind (_isadded_ _leftamount) (`/Game/MyCharacter/Blueprints/Inventory/BPC_Inventory.TryAddItem` InventoryComponent (`self.ItemObject`) true))
  (if (and _isadded_ (== _leftamount 0))
    (`self.K2_DestroyActor`)
    (else
      (`/Game/MyCharacter/Blueprints/Inventory/BP_BaseItemObject.SetAmount` (`self.ItemObject`) _leftamount))))

(fn `GetDefaultItemObject`
  (returns (ItemObject :type "/Game/MyCharacter/Blueprints/Inventory/BP_BaseItemObject Object Reference"))
  (bind (_dimension_x _dimension_y) (`KismetMathLibrary.BreakVector2D` (`self.Dimension`)))
  (bind _returnvalue (`|GenericCreateObject` self "/Game/MyCharacter/Blueprints/Inventory/BP_BaseItemObject.BP_BaseItemObject_C" (make `IntPoint` (`KismetMathLibrary.FTrunc` _dimension_x) (`KismetMathLibrary.FTrunc` _dimension_y)) (`self.Icon`) (`GameplayStatics.GetObjectClass` self) (`self.ItemInfo`) (`self.Amount`)))
  (return _returnvalue))

(fn `GetItemObject`
  (returns (ItemObject :type "/Game/MyCharacter/Blueprints/Inventory/BP_BaseItemObject Object Reference"))
  (return (`self.ItemObject`)))

(fn `UseItem`
  (params (ItemObject :type "/Game/MyCharacter/Blueprints/Inventory/BP_BaseItemObject Object Reference") (PlayerCharacter :type "/Game/MyCharacter/Blueprints/BP_MyCharacter Object Reference")))

(fn `UserConstructionScript`)